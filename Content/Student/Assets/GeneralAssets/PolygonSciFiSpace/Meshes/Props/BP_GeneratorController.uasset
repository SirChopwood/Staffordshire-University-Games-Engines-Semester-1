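; Generator controller that switches the generator effects and lighting on or off when its CubePad is activated or deactivated.
; Activation starts spark and lightning Niagara actors, then after a delay lights PointLights with "Generator" in their names and stops BP_EmergencyLight spinning.
; Deactivation does the reverse.
; Targets are found by level-wide class searches filtered by asset or object name, with Delay nodes inside the light loops.
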(event `self.ReceiveBeginPlay`
  (bind _cubepad (`self.CubePad`))
  (add `/Game/Core/Blueprints/Core/BasePowerObjects/PowerSwitch.OnActivated` _cubepad (delegate `Turn on the lights!`))
  (add `/Game/Core/Blueprints/Core/BasePowerObjects/PowerSwitch.OnDeactivated` _cubepad (delegate `Bravo Six going Dark`)))

(event `Turn on the lights!`
  (params (Sender :type "Actor Object Reference"))
  (bind _outactors (`GameplayStatics.GetAllActorsOfClass` "/Script/Niagara.NiagaraActor"))
  (for _array_element _outactors
    (bind _niagaracomponent (`NiagaraActor.NiagaraComponent` _array_element))
    (bind _returnvalue (`NiagaraComponent.GetAsset` _niagaracomponent))
    (if (or (== _returnvalue "/Game/Student/Submission/Particles/NS_Sparks_Generator.NS_Sparks_Generator") (== _returnvalue "/Game/Student/Submission/Particles/NS_Lightning.NS_Lightning"))
      (`ActorComponent.Activate` _niagaracomponent false)))
  (`KismetSystemLibrary.Delay` 3.0)
  (bind _outactors_2 (`GameplayStatics.GetAllActorsOfClass` "/Script/Engine.PointLight"))
  (for _array_element_2 _outactors_2
    (if (`KismetStringLibrary.Contains` (`KismetSystemLibrary.GetObjectName` _array_element_2) "Generator")
      (`LightComponent.SetIntensity` (`PointLight.PointLightComponent` _array_element_2) 1.0)
      (`KismetSystemLibrary.Delay` 0.3)
      (bind _outactors_3 (`GameplayStatics.GetAllActorsOfClass` "/Game/Student/Assets/GeneralAssets/PolygonSciFiSpace/Meshes/Props/BP_EmergencyLight.BP_EmergencyLight_C"))
      (for _array_element_3 _outactors_3
        (set `/Game/Student/Assets/GeneralAssets/PolygonSciFiSpace/Meshes/Props/BP_EmergencyLight.Spin` false _array_element_3)
        (`KismetSystemLibrary.Delay` 0.3)))))

(event `Bravo Six going Dark`
  (params (Sender :type "Actor Object Reference"))
  (bind _outactors (`GameplayStatics.GetAllActorsOfClass` "/Script/Niagara.NiagaraActor"))
  (for _array_element _outactors
    (bind _niagaracomponent (`NiagaraActor.NiagaraComponent` _array_element))
    (bind _returnvalue (`NiagaraComponent.GetAsset` _niagaracomponent))
    (if (or (== _returnvalue "/Game/Student/Submission/Particles/NS_Sparks_Generator.NS_Sparks_Generator") (== _returnvalue "/Game/Student/Submission/Particles/NS_Lightning.NS_Lightning"))
      (`ActorComponent.Deactivate` _niagaracomponent)))
  (`KismetSystemLibrary.Delay` 3.0)
  (bind _outactors_2 (`GameplayStatics.GetAllActorsOfClass` "/Script/Engine.PointLight"))
  (for _array_element_2 _outactors_2
    (if (`KismetStringLibrary.Contains` (`KismetSystemLibrary.GetObjectName` _array_element_2) "Generator")
      (`LightComponent.SetIntensity` (`PointLight.PointLightComponent` _array_element_2) 0.0)
      (`KismetSystemLibrary.Delay` 0.3)
      (bind _outactors_3 (`GameplayStatics.GetAllActorsOfClass` "/Game/Student/Assets/GeneralAssets/PolygonSciFiSpace/Meshes/Props/BP_EmergencyLight.BP_EmergencyLight_C"))
      (for _array_element_3 _outactors_3
        (set `/Game/Student/Assets/GeneralAssets/PolygonSciFiSpace/Meshes/Props/BP_EmergencyLight.Spin` true _array_element_3)
        (`KismetSystemLibrary.Delay` 0.3)))))

(fn `UserConstructionScript`)