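; Game mode for timed puzzle levels, running pre-game, play and end states through event dispatchers.
; On BeginPlay it finds or spawns the FlythroughManager and EndGoal, deriving gold, silver and bronze times from the goal's target time.
; The flythrough's end starts the timer and UI; reaching the goal records completion time, freezes the player and plays the end sequence.
; Helper functions report elapsed time and current reward tier.
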(event `self.ReceiveBeginPlay`
  ;[1 1 1] Begin Play
  (add `self.OnPreGame` (`|CreateDelegate` :!event `PreGame`))
  (add `self.OnStartGame` (`|CreateDelegate` :!event `StartGame`))
  (add `self.OnEndGame` (`|CreateDelegate` :!event `EndGame`))
  (bind _outactors (`GameplayStatics.GetAllActorsOfClass` "/Game/Framework/Gameplay/Required/FlythroughManager.FlythroughManager_C"))
  (bind _output (`|GetArrayItem` _outactors))
  (`/Engine/EditorBlueprintResources/StandardMacros.IsValid` _output
    (:`Is Valid`
      (set `self.FlythroughManager` _output))
    (:`Is Not Valid`
      (bind _returnvalue (`|SpawnActorFromClass` "/Game/Framework/Gameplay/Required/FlythroughManager.FlythroughManager_C" (`KismetMathLibrary.MakeTransform` (0.0 0.0 0.0)) "Undefined" "OverrideRootScale" null null))
      (set `self.FlythroughManager` _returnvalue)))
  (bind _outactors_2 (`GameplayStatics.GetAllActorsOfClass` "/Game/Framework/Gameplay/Required/EndGoal.EndGoal_C"))
  (bind _output_2 (`|GetArrayItem` _outactors_2))
  (`/Engine/EditorBlueprintResources/StandardMacros.IsValid` _output_2
    (:`Is Valid`
      (set `self.EndGoal` _output_2))
    (:`Is Not Valid`
      (bind _returnvalue_2 (`|SpawnActorFromClass` "/Game/Framework/Gameplay/Required/EndGoal.EndGoal_C" (`KismetMathLibrary.MakeTransform` (0.0 0.0 0.0)) "Undefined" "OverrideRootScale" null null))
      (set `self.EndGoal` _returnvalue_2)))
  (set `self.TargetTime` (`/Game/Framework/Gameplay/Required/EndGoal.TargetTime` (`self.EndGoal`)))
  (`self.SetTimes`)
  (`self.OnPreGame`))

(event `PreGame`
  ;[1 1 1] Match States
  (set `self.MatchState` "NewEnumerator0")
  (`/Engine/EditorBlueprintResources/StandardMacros.IsValid` (`self.FlythroughManager`)
    (:`Is Valid`
      (add `/Game/Framework/Gameplay/Required/FlythroughManager.OnSequenceEnd` (`self.FlythroughManager`) (`|CreateDelegate` :!event `FlythroughEnd`))
      (`/Game/Core/Blueprints/Core/I_Init.Init` (`self.FlythroughManager`))
      (`/Engine/EditorBlueprintResources/StandardMacros.IsValid` (`self.EndGoal`)
        (:`Is Valid`
          (add `/Game/Framework/Gameplay/Required/EndGoal.OnGoalReached` (`self.EndGoal`) (`|CreateDelegate` :!event `GoalReached`)))))))

(event `SetTimes`
  (bind _targettime (`self.TargetTime`))
  (bind _targettime_2 (`self.TargetTime`))
  ;[1 1 1] Time
  (set `self.GoldTime` (`self.TargetTime`))
  (set `self.SilverTime` (+ _targettime_2 (* _targettime_2 (- 1.0 0.66))))
  (set `self.BronzeTime` (+ _targettime (* _targettime (- 1.0 0.33)))))

(event `StartGame`
  ;[1 1 1] Match States
  (set `self.MatchState` "NewEnumerator1")
  (set `self.StartTime` (`GameplayStatics.GetTimeSeconds`))
  (bind _returnvalue (`|CreateWidget` "/Game/Core/Blueprints/UI/UIManager.UIManager_C" (`GameplayStatics.GetPlayerController` 0)))
  (`UserWidget.AddToPlayerScreen` _returnvalue 0)
  (set `self.UIManager` _returnvalue))

(event `EndGame`
  ;[1 1 1] Match States
  (set `self.MatchState` "NewEnumerator2")
  (`MovementComponent.StopMovementImmediately` (`Character.CharacterMovement` (`GameplayStatics.GetPlayerCharacter` 0)))
  (`self.DisableInput` (`GameplayStatics.GetPlayerCharacter` 0) (`GameplayStatics.GetPlayerController` 0))
  (`/Game/Framework/Gameplay/Required/FlythroughManager.PlayEndSequence` (`self.FlythroughManager`) (`self.TargetTime`) (`self.CompleteTime`))
  (`Widget.RemoveFromParent` (`self.UIManager`)))

(event `TryStartGame`
  ;[1 1 1] Game Rules
  (bind _canstart (`self.CanStartGame`))
  (if _canstart
    (`self.OnStartGame`)))

(event `FlythroughEnd`
  ;[1 1 1] Gameplay Events
  (`self.TryStartGame`))

(event `GoalReached`
  (params (CompleteTime :type "Float (double-precision)"))
  (bind _returnvalue (- CompleteTime (`self.StartTime`)))
  ;[1 1 1] Gameplay Events
  (set `self.CompleteTime` (`KismetMathLibrary.SelectFloat` _returnvalue 0.0 (> _returnvalue 0.0)))
  (`self.TryEndGame`))

(event `TryEndGame`
  ;[1 1 1] Game Rules
  (bind _canend (`self.CanEndGame`))
  (if _canend
    (`self.OnEndGame`)))

(fn `CanEndGame`
  (returns (CanEnd :type Boolean))
  (return (> (`self.CompleteTime`) 0.0)))

(fn `CanStartGame`
  (returns (CanStart :type Boolean))
  (`/Engine/EditorBlueprintResources/StandardMacros.IsValid` (`self.EndGoal`)
    (:`Is Valid`
      (return true))
    (:`Is Not Valid`
      (return false))))

(fn `GetCurrentRewardLevel`
  (returns (RewardLevel :type "/Game/Core/Blueprints/Core/RewardLevels Enum"))
  (if (<= (`self.GetCurrentTime`) (`self.GoldTime`))
    (return "NewEnumerator0")
    (elif (<= (`self.GetCurrentTime`) (`self.SilverTime`))
      (return "NewEnumerator1")
      (elif (<= (`self.GetCurrentTime`) (`self.BronzeTime`))
        (return "NewEnumerator2")
        (else
          (return "NewEnumerator3"))))))

(fn `GetCurrentTime`
  (returns (Time :type "Float (double-precision)"))
  (return (- (`GameplayStatics.GetTimeSeconds`) (`self.StartTime`))))

(fn `GetTimeIntoCurrentRewardLevel`
  (returns (Time :type "Float (double-precision)"))
  (switch `/Game/Core/Blueprints/Core/RewardLevels` (`self.GetCurrentRewardLevel`)
    (:`NewEnumerator0`
      (return (`self.GetCurrentTime`)))
    (:`NewEnumerator1`
      (return (- (`self.GetCurrentTime`) (`self.GoldTime`))))
    (:`NewEnumerator2`
      (return (- (`self.GetCurrentTime`) (`self.SilverTime`))))
    (:`NewEnumerator3`
      (return (- (`self.GetCurrentTime`) (`self.BronzeTime`))))))

(fn `UserConstructionScript`)