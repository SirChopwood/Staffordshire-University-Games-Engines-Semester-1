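; InteractComponent highlights the actor currently targeted for interaction with a colored outline.
; Init creates a dynamic outline material and applies it as a blendable on an unbound post-process volume passed in.
; StartInteract clears any previous target, enables custom depth and stencil on the new target's static meshes, and sets the outline color parameter.
; EndInteract disables those depth flags, zeroes the color and clears the target.
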(event `Init`
  (params (PostProcess :type "PostProcessComponent Object Reference"))
  ;[1 1 1] Init
  (bind _returnvalue (`KismetMaterialLibrary.CreateDynamicMaterialInstance` (`self.OutlineMaterial`)))
  (set `self.PPInst` _returnvalue)
  (set `PostProcessComponent.bUnbound` true PostProcess)
  (set `PostProcessComponent.Settings` (make `PostProcessSettings` :`WeightedBlendables` (make `WeightedBlendables` (`|MakeArray` (make `WeightedBlendable` 1.0 (`self.PPInst`))))) PostProcess))

(event `StartInteract`
  (params (Target :type "Actor Object Reference") (Value :type "LinearColor Structure"))
  ;[1 1 1] Interaction
  (`/Engine/EditorBlueprintResources/StandardMacros.IsValid` (`self.InteractObject`)
    (:`Is Valid`
      (if (not (== Target (`self.InteractObject`)))
        (`self.EndInteract`)
        (set `self.InteractObject` Target :!label _label)
        (for _array_element (`Actor.K2_GetComponentsByClass` Target "/Script/Engine.StaticMeshComponent")
          (`PrimitiveComponent.SetRenderCustomDepth` _array_element true)
          (`PrimitiveComponent.SetCustomDepthStencilValue` _array_element 1))))
    (:`Is Not Valid`
      (goto _label)))
  (`MaterialInstanceDynamic.SetVectorParameterValue` (`self.PPInst`) (`self.OutlineParamName`) Value))

(event `EndInteract`
  ;[1 1 1] Interaction
  (`/Engine/EditorBlueprintResources/StandardMacros.IsValid` (`self.InteractObject`)
    (:`Is Valid`
      (for _array_element (`Actor.K2_GetComponentsByClass` (`self.InteractObject`) "/Script/Engine.StaticMeshComponent")
        (`PrimitiveComponent.SetRenderCustomDepth` _array_element false)
        (`PrimitiveComponent.SetCustomDepthStencilValue` _array_element 0))
      (`MaterialInstanceDynamic.SetVectorParameterValue` :`self` (`self.PPInst`) :`ParameterName` (`self.OutlineParamName`))
      (set `self.InteractObject` null))))