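; RespawnHelper is a short-lived actor that spawns a replacement actor after a delay, using its RespawnInfo data.
; BeginPlay starts a one-shot timer for the configured respawn time.
; The Respawn event spawns the stored class at the saved transform, copies the respawn time into the new actor's RespawnComponent, then destroys the helper.
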(event `self.ReceiveBeginPlay`
  (`self.StartRespawn`))

(event `StartRespawn`
  (bind (_respawninfo_class _respawninfo_spawntransform _respawninfo_respawntime) (break `/Game/Core/Blueprints/Core/RespawnInfo` (`self.RespawnInfo`)))
  (`KismetSystemLibrary.K2_SetTimerDelegate` (`|CreateDelegate` :!event `Respawn`) _respawninfo_respawntime))

(event `Respawn`
  (bind (_respawninfo_class _respawninfo_spawntransform _respawninfo_respawntime) (break `/Game/Core/Blueprints/Core/RespawnInfo` (`self.RespawnInfo`)))
  (bind _returnvalue (`|SpawnActorFromClass` _respawninfo_class _respawninfo_spawntransform "Undefined" "OverrideRootScale" null null))
  (set `/Game/Core/Blueprints/Core/RespawnComponent.RespawnTime` _respawninfo_respawntime (`self.GetComponentByClass` _returnvalue "/Game/Core/Blueprints/Core/RespawnComponent.RespawnComponent_C"))
  (`self.K2_DestroyActor`))

(fn `UserConstructionScript`)