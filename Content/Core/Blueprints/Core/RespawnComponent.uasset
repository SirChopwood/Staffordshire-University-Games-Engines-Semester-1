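; Actor component that lets its owner respawn after it leaves play.
; It stores the owner's transform at BeginPlay, and an event can replace that saved transform.
; On EndPlay, if Respawnable is set, it spawns a separate RespawnHelper actor, passing it the owner's class, saved transform and respawn time.
; EndPlay reason is not checked, so any end of play triggers the spawn.
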(event `self.ReceiveBeginPlay`
  (set `self.RespawnTransform` (`Actor.GetTransform` (`self.GetOwner`))))

(event `/Game/Core/Blueprints/Core/I_Respawn.UpdateRespawnTransform`
  (params (RespawnTransform :type "Transform Structure"))
  (set `self.RespawnTransform` RespawnTransform))

(event `self.ReceiveEndPlay`
  (params (EndPlayReason :type "EEndPlayReason Enum" :default "Destroyed"))
  (if (`self.Respawnable`)
    (`|SpawnActorFromClass` "/Game/Core/Blueprints/Core/RespawnHelper.RespawnHelper_C" (`KismetMathLibrary.MakeTransform` (0.0 0.0 0.0)) "Undefined" "OverrideRootScale" null (make `/Game/Core/Blueprints/Core/RespawnInfo` (`GameplayStatics.GetObjectClass` (`self.GetOwner`)) (`self.RespawnTransform`) (`self.RespawnTime`)) null)))